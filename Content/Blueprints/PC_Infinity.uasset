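; PC_Infinity is a player controller that sets up the game's UI widgets and handles pausing.
; On BeginPlay it creates and stores the main UI, pause menu and game over widgets, adding only the main UI to the viewport.
; The Pause input drives a FlipFlop that alternately shows or removes the pause menu, along with game pause and mouse cursor.
; GetPlayerControllerRef returns the controller itself.
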(event `self.ReceiveBeginPlay`
  (bind _returnvalue (`|CreateWidget` "/Game/UI/WB_MainUI.WB_MainUI_C"))
  (bind _output_get (set `self.WB_MainUI` _returnvalue))
  (`UserWidget.AddToViewport` _output_get 0)
  (bind _returnvalue_2 (`|CreateWidget` "/Game/UI/WB_Pause_Menu.WB_Pause_Menu_C"))
  (set `self.WB_PauseMenu` _returnvalue_2)
  (bind _returnvalue_3 (`|CreateWidget` "/Game/UI/WB_GameOver.WB_GameOver_C"))
  (set `self.WB_GameOver` _returnvalue_3))

(event `InputAction|Pause` :paused true
  (params (Key :type "Key Structure"))
  (bind _wb_pausemenu (`self.WB_PauseMenu`))
  (:`Pressed`
    (`/Engine/EditorBlueprintResources/StandardMacros.FlipFlop`
      (:`A`
        (`UserWidget.AddToViewport` _wb_pausemenu 0)
        (`GameplayStatics.SetGamePaused` true)
        (set `self.bShowMouseCursor` true))
      (:`B`
        (`Widget.RemoveFromParent` _wb_pausemenu)
        (`GameplayStatics.SetGamePaused` false)
        (set `self.bShowMouseCursor` false)))))

(fn `GetPlayerControllerRef`
  (returns (PlayerControllerRef :type "/Game/Blueprints/PC_Infinity Object Reference"))
  (return self))

(fn `UserConstructionScript`)