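; Endless-runner floor tile that exposes an attach transform for chaining tiles and fills itself with random content on construction.
; The construction script randomly picks obstacles or pickups, adding child actors at one of three obstacle points or at random points inside the pickup area box.
; When the player overlaps NextTileCollision, it asks the game mode to spawn another tile, then destroys itself after a short delay.
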(event `self.NextTileCollision.OnComponentBeginOverlap`
  (params (OverlappedComponent :type "PrimitiveComponent Object Reference") (OtherActor :type "Actor Object Reference") (OtherComp :type "PrimitiveComponent Object Reference") (OtherBodyIndex :type Integer) (bFromSweep :type Boolean) (SweepResult :type "HitResult Structure (by ref)"))
  (if (`self.ActorHasTag` OtherActor "Player")
    (bind _gamemoderef (message `/Game/Blueprints/Interfaces/INT_GameMode.GetGameModeRef` (`GameplayStatics.GetGameMode`)))
    (`/Game/Blueprints/GM_Infinity.Spawn Floor Tile` _gamemoderef)
    (`KismetSystemLibrary.Delay` 1.5)
    (`self.K2_DestroyActor`)))

(fn `GetAttachLocation`
  (returns (AttachLocation :type "Transform Structure"))
  (return (`SceneComponent.K2_GetComponentToWorld` (`self.AttachPoint`))))

(fn `GetFloorTileRef`
  (returns (FloorTileRef :type "/Game/Blueprints/Tiles/BP_FloorTile Object Reference"))
  (return self))

(fn `SetSpawnPoints`
  (set `self.SpawnPoints` (`|MakeArray` (`SceneComponent.GetRelativeTransform` (`self.ObstacleSpawnPoint`)) (`SceneComponent.GetRelativeTransform` (`self.ObstacleSpawnPointL`)) (`SceneComponent.GetRelativeTransform` (`self.ObstacleSpawnPointR`))))
  (return))

(fn `Spawn Obstacle`
  (switch `int` (`KismetMathLibrary.RandomIntegerInRange` 0 3)
    (:`Default`
      (`AddComponent|NODE_AddChildActorComponent-0` :`RelativeTransform` (`KismetArrayLibrary.Array_Random` (`self.SpawnPoints`)) :!label _label))
    (:`0`
      (goto _label))
    (:`1`
      (`AddComponent|NODE_AddChildActorComponent-3` :`RelativeTransform` (`KismetArrayLibrary.Array_Random` (`self.SpawnPoints`))))
    (:`2`
      (`AddComponent|NODE_AddChildActorComponent-6` :`RelativeTransform` (`KismetArrayLibrary.Array_Random` (`self.SpawnPoints`))))
    (:`3`
      (`AddComponent|NODE_AddChildActorComponent-7` :`RelativeTransform` (`SceneComponent.GetRelativeTransform` (`self.ObstacleSpawnPoint`))))))

(fn `SpawnPickup`
  (bind _pickuparea (`self.PickupArea`))
  (bind _pickuparea_2 (`self.PickupArea`))
  (bind _pickuparea_3 (`self.PickupArea`))
  (switch `int` (`KismetMathLibrary.RandomIntegerInRange` 0 4)
    (:`Default`
      (for _ (range 3) :!label _label
        (`AddComponent|NODE_AddChildActorComponent-1` :`RelativeTransform` (`KismetMathLibrary.Conv_VectorToTransform` (`KismetMathLibrary.RandomPointInBoundingBox` (`SceneComponent.RelativeLocation` _pickuparea_2) (`BoxComponent.BoxExtent` _pickuparea_2))))))
    (:`0`
      (goto _label))
    (:`1`
      (goto _label))
    (:`2`
      (goto _label))
    (:`3`
      (`AddComponent|NODE_AddChildActorComponent-4` :`RelativeTransform` (`KismetMathLibrary.Conv_VectorToTransform` (`KismetMathLibrary.RandomPointInBoundingBox` (`SceneComponent.RelativeLocation` _pickuparea) (`BoxComponent.BoxExtent` _pickuparea)))))
    (:`4`
      (`AddComponent|NODE_AddChildActorComponent-5` :`RelativeTransform` (`KismetMathLibrary.Conv_VectorToTransform` (`KismetMathLibrary.RandomPointInBoundingBox` (`SceneComponent.RelativeLocation` _pickuparea_3) (`BoxComponent.BoxExtent` _pickuparea_3)))))))

(fn `UserConstructionScript`
  (`self.SetSpawnPoints`)
  (switch `int` (`KismetMathLibrary.RandomIntegerInRange` 0 1)
    (:`Default`
      (`self.Spawn Obstacle` :!label _label))
    (:`0`
      (goto _label))
    (:`1`
      (`self.SpawnPickup`))))