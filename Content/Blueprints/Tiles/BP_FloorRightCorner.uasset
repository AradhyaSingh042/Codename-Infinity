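; BP_FloorRightCorner is a right-corner floor tile with a turn zone and two walls that kill the player on impact.
; Wall hits from actors tagged "Player" fetch the player reference from player character 0 through GetPlayerRefMessage, then send it PlayerDeathMessage.
; TurnZone overlap by the player only fetches that reference and does nothing further with it.
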(event `self.ReceiveBeginPlay`)

(event `self.TurnZone.OnComponentBeginOverlap`
  (params (OverlappedComponent :type "PrimitiveComponent Object Reference") (OtherActor :type "Actor Object Reference") (OtherComp :type "PrimitiveComponent Object Reference") (OtherBodyIndex :type Integer) (bFromSweep :type Boolean) (SweepResult :type "HitResult Structure (by ref)"))
  (if (`self.ActorHasTag` OtherActor "Player")
    (message `/Game/Blueprints/Interfaces/INT_PlayerBase.GetPlayerRef` (`GameplayStatics.GetPlayerCharacter` 0))))

(event `self.Wall1.OnComponentHit`
  (params (HitComponent :type "PrimitiveComponent Object Reference") (OtherActor :type "Actor Object Reference") (OtherComp :type "PrimitiveComponent Object Reference") (NormalImpulse :type "Vector Structure") (Hit :type "HitResult Structure (by ref)"))
  (if (`self.ActorHasTag` OtherActor "Player")
    (bind _playerref (message `/Game/Blueprints/Interfaces/INT_PlayerBase.GetPlayerRef` (`GameplayStatics.GetPlayerCharacter` 0)))
    (message `/Game/Blueprints/Interfaces/INT_PlayerBase.PlayerDeath` _playerref)))

(event `self.Wall2.OnComponentHit`
  (params (HitComponent :type "PrimitiveComponent Object Reference") (OtherActor :type "Actor Object Reference") (OtherComp :type "PrimitiveComponent Object Reference") (NormalImpulse :type "Vector Structure") (Hit :type "HitResult Structure (by ref)"))
  (if (`self.ActorHasTag` OtherActor "Player")
    (bind _playerref (message `/Game/Blueprints/Interfaces/INT_PlayerBase.GetPlayerRef` (`GameplayStatics.GetPlayerCharacter` 0)))
    (message `/Game/Blueprints/Interfaces/INT_PlayerBase.PlayerDeath` _playerref)))

(fn `UserConstructionScript`)