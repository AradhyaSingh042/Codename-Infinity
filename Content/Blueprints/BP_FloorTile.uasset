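; BP_FloorTile is an endless-runner floor segment that populates itself and chains to the next tile.
; Construction randomly adds either one obstacle at one of three spawn points or three pickups at random points inside PickupArea, as child actors.
; When the player overlaps NextTileCollision, it asks the game mode to spawn another tile, then destroys itself after a short delay.
; GetAttachLocation exposes the AttachPoint transform.
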(event `self.NextTileCollision.OnComponentBeginOverlap`
  (params (OverlappedComponent :type "PrimitiveComponent Object Reference") (OtherActor :type "Actor Object Reference") (OtherComp :type "PrimitiveComponent Object Reference") (OtherBodyIndex :type Integer) (bFromSweep :type Boolean) (SweepResult :type "HitResult Structure (by ref)"))
  (if (`self.ActorHasTag` OtherActor "Player")
    (bind _gamemoderef (message `/Game/Blueprints/INT_GameMode.GetGameModeRef` (`GameplayStatics.GetGameMode`)))
    (`/Game/Blueprints/GM_Infinity.Spawn Floor Tile` _gamemoderef)
    (`KismetSystemLibrary.Delay` 1.5)
    (`self.K2_DestroyActor`)))

(fn `GetAttachLocation`
  (returns (AttachLocation :type "Transform Structure"))
  (return (`SceneComponent.K2_GetComponentToWorld` (`self.AttachPoint`))))

(fn `GetFloorTileRef`
  (returns (FloorTileRef :type "/Game/Blueprints/BP_FloorTile Object Reference"))
  (return self))

(fn `SetSpawnPoints`
  (set `self.SpawnPoints` (`|MakeArray` (`SceneComponent.GetRelativeTransform` (`self.ObstacleSpawnPoint`)) (`SceneComponent.GetRelativeTransform` (`self.ObstacleSpawnPointL`)) (`SceneComponent.GetRelativeTransform` (`self.ObstacleSpawnPointR`))))
  (return))

(fn `SpawnObstacle`
  (`AddComponent|NODE_AddChildActorComponent-0` :`RelativeTransform` (`KismetArrayLibrary.Array_Random` (`self.SpawnPoints`))))

(fn `SpawnPickup`
  (bind _pickuparea (`self.PickupArea`))
  (`AddComponent|NODE_AddChildActorComponent-1` :`RelativeTransform` (`KismetMathLibrary.Conv_VectorToTransform` (`KismetMathLibrary.RandomPointInBoundingBox` (`SceneComponent.RelativeLocation` _pickuparea) (`BoxComponent.BoxExtent` _pickuparea)))))

(fn `UserConstructionScript`
  (`self.SetSpawnPoints`)
  (switch `int` (`KismetMathLibrary.RandomIntegerInRange` 0 1)
    (:`Default`
      (`self.SpawnObstacle` :!label _label))
    (:`0`
      (goto _label))
    (:`1`
      (for _ (range 3)
        (`self.SpawnPickup`)))))