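; BP_NewCustomRunes is a collectible rune that animates in place and raises the player's score when picked up.
; A timeline drives the mesh's relative X and Z position, seeded at a random time to vary its phase and replayed whenever it finishes.
; On overlap with a "Player"-tagged actor, it increments score through the player character's reference, plays a star sound and destroys itself.
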(event `self.ReceiveBeginPlay`
  (`|ExecutionSequence`
    (:`then_0`
      (bind (_direction _position) (`Timeline|Timeline_0` :`NewTime` (`KismetMathLibrary.RandomFloatInRange` 0.0 10.0) :!via `SetNewTime` :!label _label)
        (:`Update`
          (`SceneComponent.K2_SetRelativeLocation` (`self.StaticMesh`) (* _position (10.0 0.0 20.0)) false false))
        (:`Finished`
          (`|ExecutionSequence`
            (:`then_0`
              (goto _label :!via `PlayFromStart`))))))
    (:`then_1`
      (goto _label))))

(event `self.StaticMesh.OnComponentBeginOverlap`
  (params (OverlappedComponent :type "PrimitiveComponent Object Reference") (OtherActor :type "Actor Object Reference") (OtherComp :type "PrimitiveComponent Object Reference") (OtherBodyIndex :type Integer) (bFromSweep :type Boolean) (SweepResult :type "HitResult Structure (by ref)"))
  (if (`self.ActorHasTag` OtherActor "Player")
    (bind _playerref (message `/Game/Blueprints/INT_PlayerBase.GetPlayerRef` (`GameplayStatics.GetPlayerCharacter` 0)))
    (`/Game/Blueprints/BP_PlayerBase.IncrementScore` _playerref)
    (`GameplayStatics.PlaySoundAtLocation` "/Game/Assets/SFX_StarCue.SFX_StarCue" (`self.K2_GetActorLocation`) (struct) 1.0 1.0 0.0 null null null)
    (`self.K2_DestroyActor`)))

(fn `UserConstructionScript`)