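; A collectible rune pickup that increments the player's score on contact, plays a coin sound and destroys itself.
; The mesh bobs on a timeline started at a random time, so separate runes move out of sync.
; If the player's magnet is active, entering MagnetZone interpolates the rune toward the player through a second timeline.
; That path scores immediately and destroys the rune after a short delay, without playing the sound itself.
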(event `self.ReceiveBeginPlay`
  (`|ExecutionSequence`
    (:`then_0`
      (bind (_direction _position) (`Timeline|Timeline_0` :`NewTime` (`KismetMathLibrary.RandomFloatInRange` 0.0 10.0) :!via `SetNewTime` :!label _label)
        (:`Update`
          (`SceneComponent.K2_SetRelativeLocation` (`self.StaticMesh`) (* _position (10.0 0.0 20.0)) false false))
        (:`Finished`
          (`|ExecutionSequence`
            (:`then_0`
              (goto _label :!via `PlayFromStart`))))))
    (:`then_1`
      (goto _label))))

(event `self.StaticMesh.OnComponentBeginOverlap`
  (params (OverlappedComponent :type "PrimitiveComponent Object Reference") (OtherActor :type "Actor Object Reference") (OtherComp :type "PrimitiveComponent Object Reference") (OtherBodyIndex :type Integer) (bFromSweep :type Boolean) (SweepResult :type "HitResult Structure (by ref)"))
  (if (`self.ActorHasTag` OtherActor "Player")
    (bind _playerref (message `/Game/Blueprints/Interfaces/INT_PlayerBase.GetPlayerRef` (`GameplayStatics.GetPlayerCharacter` 0)))
    (`/Game/Blueprints/BP_PlayerBase.IncrementScore` _playerref)
    (`GameplayStatics.PlaySoundAtLocation` "/Game/InterfaceAndItemSounds/Cues/Coins_04_wav_Cue.Coins_04_wav_Cue" (`self.K2_GetActorLocation`) (struct) 1.0 1.0 0.0 null null null)
    (`self.K2_DestroyActor`)))

(event `self.MagnetZone.OnComponentBeginOverlap`
  (params (OverlappedComponent :type "PrimitiveComponent Object Reference") (OtherActor :type "Actor Object Reference") (OtherComp :type "PrimitiveComponent Object Reference") (OtherBodyIndex :type Integer) (bFromSweep :type Boolean) (SweepResult :type "HitResult Structure (by ref)"))
  (if (`self.ActorHasTag` OtherActor "Player")
    (bind _playerref (message `/Game/Blueprints/Interfaces/INT_PlayerBase.GetPlayerRef` (`GameplayStatics.GetPlayerCharacter` 0)))
    (if (`/Game/Blueprints/BP_PlayerBase.MagnetActive` _playerref)
      (`|ExecutionSequence`
        (:`then_0`
          (bind (_direction _vectoralpha) (`Timeline|MagnetTimeline` :!via `PlayFromStart`)
            (:`Update`
              (`self.K2_SetActorLocation` (+ _vectoralpha (`KismetMathLibrary.VInterpTo` (`self.K2_GetActorLocation`) (`self.K2_GetActorLocation` (`GameplayStatics.GetPlayerCharacter` 0)) (`GameplayStatics.GetWorldDeltaSeconds`) 6.0))))))
        (:`then_1`
          (bind _playerref_2 (message `/Game/Blueprints/Interfaces/INT_PlayerBase.GetPlayerRef` (`GameplayStatics.GetPlayerCharacter` 0)))
          (`/Game/Blueprints/BP_PlayerBase.IncrementScore` _playerref_2)
          (`KismetSystemLibrary.Delay` 0.3)
          (`self.K2_DestroyActor`))))))

(fn `UserConstructionScript`)