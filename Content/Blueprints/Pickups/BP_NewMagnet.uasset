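; BP_NewMagnet is a magnet pickup that switches on the player's magnet state when touched.
; On overlap with a Player-tagged actor, it fetches player 0's reference through a message call, sets MagnetActive, hides the Magnet component and plays a sound.
; It then immediately calls DeactivateMagnetMessage on the player, leaving deactivation to that side.
; The pickup is only hidden, with no destroy or collision change.
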(event `self.Magnet.OnComponentBeginOverlap`
  (params (OverlappedComponent :type "PrimitiveComponent Object Reference") (OtherActor :type "Actor Object Reference") (OtherComp :type "PrimitiveComponent Object Reference") (OtherBodyIndex :type Integer) (bFromSweep :type Boolean) (SweepResult :type "HitResult Structure (by ref)"))
  (if (`self.ActorHasTag` OtherActor "Player")
    (bind _playerref (message `/Game/Blueprints/Interfaces/INT_PlayerBase.GetPlayerRef` (`GameplayStatics.GetPlayerCharacter` 0)))
    (set `self.PlayerRef` _playerref)
    (set `/Game/Blueprints/BP_PlayerBase.MagnetActive` true _playerref)
    (`SceneComponent.SetVisibility` (`self.Magnet`) false false)
    (`GameplayStatics.PlaySoundAtLocation` "/Game/Assets/SFX_StarCue.SFX_StarCue" (`self.K2_GetActorLocation`) (struct) 1.0 1.0 0.0 null null null)
    (message `/Game/Blueprints/Interfaces/INT_PlayerBase.DeactivateMagnet` (`self.PlayerRef`))))

(fn `UserConstructionScript`)