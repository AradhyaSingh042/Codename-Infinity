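; BP_Booster is a speed boost pickup that also lets the player pass through obstacles.
; When a Player-tagged actor overlaps it, it hides the mesh, plays a sound and raises the player's walk speed.
; It disables death zone and obstacle collision on every BP_Obstacle, passing the prior speed to the player's DeactivateBoosterMessage once per obstacle.
; The pickup is only hidden, with its own collision left unchanged.
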(event `self.Booster.OnComponentBeginOverlap`
  (params (OverlappedComponent :type "PrimitiveComponent Object Reference") (OtherActor :type "Actor Object Reference") (OtherComp :type "PrimitiveComponent Object Reference") (OtherBodyIndex :type Integer) (bFromSweep :type Boolean) (SweepResult :type "HitResult Structure (by ref)"))
  (bind _charactermovement (`Character.CharacterMovement` (`self.PlayerRef`)))
  (if (`self.ActorHasTag` OtherActor "Player")
    (bind _playerref (message `/Game/Blueprints/Interfaces/INT_PlayerBase.GetPlayerRef` (`GameplayStatics.GetPlayerCharacter` 0)))
    (set `self.PlayerRef` _playerref)
    (`SceneComponent.SetVisibility` (`self.Booster`) false false)
    (`GameplayStatics.PlaySoundAtLocation` "/Game/Assets/SFX_StarCue.SFX_StarCue" (`self.K2_GetActorLocation`) (struct) 1.0 1.0 0.0 null null null)
    (bind _output_get (set `self.CurrentSpeed` (`CharacterMovementComponent.MaxWalkSpeed` _charactermovement)))
    (set `CharacterMovementComponent.MaxWalkSpeed` 2500.0 _charactermovement)
    (bind _outactors (`GameplayStatics.GetAllActorsOfClass` "/Game/Blueprints/Obstacles/BP_Obstacle.BP_Obstacle_C"))
    (bind _output_get_2 (set `self.Obstacle` _outactors))
    (for _array_element _output_get_2
      (`PrimitiveComponent.SetCollisionEnabled` (`/Game/Blueprints/Obstacles/BP_Obstacle.DeathZone` _array_element) "NoCollision")
      (`PrimitiveComponent.SetCollisionEnabled` (`/Game/Blueprints/Obstacles/BP_Obstacle.Obstacle` _array_element) "NoCollision")
      (message `/Game/Blueprints/Interfaces/INT_PlayerBase.DeactivateBooster` (`self.PlayerRef`) _output_get))))

(fn `UserConstructionScript`)