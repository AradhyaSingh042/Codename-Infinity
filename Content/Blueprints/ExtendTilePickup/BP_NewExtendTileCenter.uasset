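; BP_NewExtendTileCenter is a tile with an extendable platform and a game-over area.
; Its construction script stores left, center and right arrow transforms, spawns a child-actor platform at the center one, and places a pickup offset from it.
; A player entering ExtendAreaCenter plays a timeline that drives the platform's X scale.
; A player entering GameOverArea opens Main_Map.
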(event `self.ReceiveBeginPlay`)

(event `self.ExtendAreaCenter.OnComponentBeginOverlap`
  (params (OverlappedComponent :type "PrimitiveComponent Object Reference") (OtherActor :type "Actor Object Reference") (OtherComp :type "PrimitiveComponent Object Reference") (OtherBodyIndex :type Integer) (bFromSweep :type Boolean) (SweepResult :type "HitResult Structure (by ref)"))
  (bind _extendplatform (`self.ExtendPlatform`))
  (bind (_relativescale3d_x _relativescale3d_y _relativescale3d_z) (`KismetMathLibrary.BreakVector` (`SceneComponent.RelativeScale3D` _extendplatform)))
  (if (`self.ActorHasTag` OtherActor "Player")
    (bind (_direction _extendalpha) (`Timeline|ExtendTileAlpha`)
      (:`Update`
        (`SceneComponent.SetRelativeScale3D` _extendplatform (`KismetMathLibrary.MakeVector` _extendalpha _relativescale3d_y _relativescale3d_z))))))

(event `self.GameOverArea.OnComponentBeginOverlap`
  (params (OverlappedComponent :type "PrimitiveComponent Object Reference") (OtherActor :type "Actor Object Reference") (OtherComp :type "PrimitiveComponent Object Reference") (OtherBodyIndex :type Integer) (bFromSweep :type Boolean) (SweepResult :type "HitResult Structure (by ref)"))
  (if (`self.ActorHasTag` OtherActor "Player")
    (`GameplayStatics.OpenLevel` "Main_Map")))

(fn `SetExtendTileSpawnLocation`
  (set `self.ExtendTileSpawnPoints` (`|MakeArray` (`SceneComponent.GetRelativeTransform` (`self.Left_Arrow`)) (`SceneComponent.GetRelativeTransform` (`self.Center_Arrow`)) (`SceneComponent.GetRelativeTransform` (`self.Right_Arrow`))))
  (return))

(fn `SpawnExtendablePlatform`
  (bind _returnvalue (`AddComponent|NODE_AddChildActorComponent-1` :`RelativeTransform` (`|GetArrayItem` (`self.ExtendTileSpawnPoints`) 1)))
  (set `self.ExtendPlatform` _returnvalue))

(fn `SpawnExtendPickup`
  (bind (_returnvalue_location _returnvalue_rotation _returnvalue_scale) (`KismetMathLibrary.BreakTransform` (`SceneComponent.GetRelativeTransform` (`self.ExtendPlatform`))))
  (bind _returnvalue (`AddComponent|NODE_AddChildActorComponent-2` :`RelativeTransform` (`KismetMathLibrary.MakeTransform` (`KismetMathLibrary.MakeVector` (- (.x _returnvalue_location) 100.0) (.y _returnvalue_location) (+ (.z _returnvalue_location) 100.0)) _returnvalue_rotation _returnvalue_scale)))
  (set `self.ExtendPickup` _returnvalue))

(fn `UserConstructionScript`
  (`self.SetExtendTileSpawnLocation`)
  (`self.SpawnExtendablePlatform`)
  (`self.SpawnExtendPickup`))